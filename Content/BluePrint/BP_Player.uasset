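; BP_Player is the player character, built from modular skeletal parts that follow the upper body's pose, handling garage, inventory and bag screens plus item pickup and drop.
; On BeginPlay it links controller and HUD and spawns a far-off preview actor that mirrors its modular parts.
; G, I and E drive FlipFlop menu toggles that switch cursor, movement, shooting and character state, with busy flags and delays around animations.
; E also picks up items after an inventory check.
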(event `self.ReceiveBeginPlay`
  ;[1 1 1] Event Begin Play
  (bind _asbp_player_controller (cast `/Game/BluePrint/BP_PlayerController` (`GameplayStatics.GetPlayerController` 0)))
  (bind _output_get (set `self.Player Controller Reference` _asbp_player_controller))
  (`Controller.Possess` _output_get self)
  (`/Game/BluePrint/BP_PlayerController.Refresh UI Player Reference` _output_get)
  (set `self.GameHud Reference` (`/Game/BluePrint/BP_PlayerController.GameHUDReference` _output_get))
  (`self.SpawnEquipmentPreview`)
  (`self.RefreshModularParts`))

(event `Key|G`
  (params (Key :type "Key Structure"))
  (bind _gamehud_reference (`self.GameHud Reference`))
  (bind _bisworkingarage (`self.bIsWorkInGarage`))
  (bind _garage (`/Game/Widget/GameHUD.Garage` _gamehud_reference))
  ;[1 1 1] Garage Test
  (:`Pressed`
    (`/Engine/EditorBlueprintResources/StandardMacros.FlipFlop`
      (:`A`
        (if (not _bisworkingarage)
          (`self.EnableMouse`)
          (`self.SetbIsShootable` _bisworkingarage)
          (set `self.bIsWorkInGarage` true)
          (`/Game/Widget/Garage.RefreshEquipmentInventory` _garage)
          (`/Game/Widget/GarageInventoryMenu.RefreshInventory` (`/Game/Widget/Garage.GarageInventoryMenu` _garage))
          (`self.SetCharacterState` "ECheckItems")
          ;[1 1 1] Use Inventory Menu
          (`/Game/Widget/GameHUD.HUDSwitcher` _gamehud_reference :!label _label)))
      (:`B`
        (if _bisworkingarage
          (`self.DisableMouse`)
          (`self.SetbIsShootable` _bisworkingarage)
          (set `self.bIsWorkInGarage` false)
          (`self.SetCharacterState` "EIdle")
          (`/Game/Widget/Inventory.RefreshInventory` (`/Game/Widget/GameHUD.InventoryMenu` _gamehud_reference))
          (goto _label))))))

(event `Key|I`
  (params (Key :type "Key Structure"))
  (bind _gamehud_reference (`self.GameHud Reference`))
  (bind _gamehud_reference_2 (`self.GameHud Reference`))
  ;[1 1 1] Use Inventory Menu
  (:`Pressed`
    (if (and (not (`self.bIsWorkInGarage`)) (not (`self.bIsBagOpen`)))
      (if (not (and (`self.IsDoingSomething`) (`/Game/Widget/GameHUD.IsInventoryEnable` (`self.GameHud Reference`))))
        (set `self.IsDoingSomething` true)
        (`/Engine/EditorBlueprintResources/StandardMacros.FlipFlop`
          (:`A`
            (`self.EnableMouse`)
            (bind _output_get (set `/Game/Widget/GameHUD.IsInventoryEnable` true _gamehud_reference))
            (`self.SetbIsShootable` (not _output_get))
            (`self.SetCharacterState` "ECheckItems")
            (`UserWidget.PlayAnimation` _gamehud_reference (`/Game/Widget/GameHUD.InventoryMenu_Anim` _gamehud_reference) 0.0 1 "Forward" 1.0 false)
            (`KismetSystemLibrary.Delay` 0.5))
          (:`B`
            (`UserWidget.PlayAnimation` _gamehud_reference_2 (`/Game/Widget/GameHUD.InventoryMenu_Anim` _gamehud_reference_2) 0.0 1 "Reverse" 1.0 false)
            (`KismetSystemLibrary.Delay` 0.5)
            (`self.DisableMouse`)
            (`self.SetbIsShootable` _output_get)
            (set `/Game/Widget/GameHUD.IsInventoryEnable` false (`self.GameHud Reference`))
            (`self.SetCharacterState` "EIdle")))
        (set `self.IsDoingSomething` false)))))

(event `SpawnEquipmentPreview`
  (bind _returnvalue (`|SpawnActorFromClass` "/Game/BluePrint/BP_UIPlayerPreView.BP_UIPlayerPreView_C" (`KismetMathLibrary.MakeTransform` (1000000.0 0.0 0.0)) "Undefined" "OverrideRootScale" self null))
  (bind _output_get (set `self.PreviewActor` _returnvalue))
  (`/Game/BluePrint/BP_UIPlayerPreView.SetSKM` _output_get (`self.ModularInventory`))
  (`SkeletalMeshComponent.SetAnimInstanceClass` (`/Game/BluePrint/BP_UIPlayerPreView.SKMUpperBody` _output_get) (`SkeletalMeshComponent.AnimClass` (`self.SKM_UpperBody`))))

(event `Key|E`
  (params (Key :type "Key Structure"))
  (bind _gamehud_reference (`self.GameHud Reference`))
  (bind _gamehud_reference_2 (`self.GameHud Reference`))
  (bind _gamehud_reference_3 (`self.GameHud Reference`))
  (bind _gamehud_reference_4 (`self.GameHud Reference`))
  (bind _gamehud_reference_5 (`self.GameHud Reference`))
  (bind _gamehud_reference_6 (`self.GameHud Reference`))
  ;[1 1 1] InterAction With Pickup
  (:`Pressed`
    (`/Engine/EditorBlueprintResources/StandardMacros.IsValid` (`self.Item`)
      (:`Is Valid`
        (if (`self.bIsBag`)
          ;[1 1 1] InterAction With Bag
          (bind _asbp_bag (cast `/Game/BluePrint/PickupItem/BP_Bag` (`self.Item`)))
          (`/Game/Widget/BagInventory.InitBag` (`/Game/Widget/GameHUD.BagInventoryMenu` (`self.GameHud Reference`)) _asbp_bag)
          (if (not (`self.IsDoingSomething`))
            (set `self.IsDoingSomething` true)
            (`/Engine/EditorBlueprintResources/StandardMacros.FlipFlop`
              (:`A`
                (bind _output_get (set `self.bIsBagOpen` true))
                (`self.EnableMouse`)
                (`self.SetbIsShootable` (not _output_get))
                (`self.SetCharacterState` "ECheckItems")
                (set `/Game/Widget/GameHUD.IsInventoryEnable` true _gamehud_reference_6)
                (set `/Game/Widget/GameHUD.InventoryVIsible` "Visible" _gamehud_reference_6)
                (`UserWidget.PlayAnimation` _gamehud_reference_6 (`/Game/Widget/GameHUD.InventoryMenu_Anim` _gamehud_reference_6) 0.0 1 "Forward" 1.0 false)
                (`KismetSystemLibrary.Delay` 0.5)
                (`/Game/Widget/BagInventory.Refresh Bag Inventory` (`/Game/Widget/GameHUD.BagInventoryMenu` _gamehud_reference_4))
                (set `/Game/Widget/GameHUD.BagEnable` true _gamehud_reference_4)
                (set `/Game/Widget/GameHUD.BagVisible` "Visible" _gamehud_reference_4)
                (`UserWidget.PlayAnimation` _gamehud_reference_4 (`/Game/Widget/GameHUD.BagInventory_Anim` _gamehud_reference_4) 0.0 1 "Forward" 1.0 false)
                (`KismetSystemLibrary.Delay` 0.5))
              (:`B`
                (`UserWidget.PlayAnimationReverse` _gamehud_reference_2 (`/Game/Widget/GameHUD.BagInventory_Anim` _gamehud_reference_2) 1.0 false)
                (`KismetSystemLibrary.Delay` 0.5)
                (set `/Game/Widget/GameHUD.BagVisible` "Hidden" _gamehud_reference_3)
                (bind _output_get_2 (set `/Game/Widget/GameHUD.BagEnable` false _gamehud_reference_3))
                (`UserWidget.PlayAnimation` _gamehud_reference (`/Game/Widget/GameHUD.InventoryMenu_Anim` _gamehud_reference) 0.0 1 "Reverse" 1.0 false)
                (`KismetSystemLibrary.Delay` 0.4)
                (`self.DisableMouse`)
                (`self.SetbIsShootable` (not _output_get_2))
                (`self.SetCharacterState` "EIdle")
                (set `/Game/Widget/GameHUD.IsInventoryEnable` false _gamehud_reference_5)
                (set `/Game/Widget/GameHUD.InventoryVIsible` "Hidden" _gamehud_reference_5)
                (set `self.bIsBagOpen` false)))
            (set `self.IsDoingSomething` false))
          (else
            (`KismetSystemLibrary.PrintString` "This is Pickup Item")
            (bind _inventoryhasspace (`/Game/BluePrint/BP_PlayerController.Inventory Check` (`self.Player Controller Reference`)))
            (if _inventoryhasspace
              (`KismetSystemLibrary.PrintString` "BP_Player : Call Pickup in Player start")
              (bind _asbp_pickup (cast `/Game/BluePrint/PickupItem/BP_Pickup` (`self.Item`)))
              (`/Game/BluePrint/PickupItem/BP_Pickup.CallPickUp` _asbp_pickup)
              (else
                (`KismetSystemLibrary.PrintString` "BP_player : inventory length is over")))))))))

(event `self.ReceiveDestroyed`
  (`self.K2_DestroyActor` (`self.PreviewActor`)))

(event `/Game/BluePrint/BP_ActionInterface.Drop Action`
  (params (`DataTable To Drop` :type "DataTableRowHandle Structure"))
  ;[1 1 1] Drop Item
  (`|SpawnActorFromClass` "/Game/BluePrint/PickupItem/BP_Pickup.BP_Pickup_C" (`SceneComponent.K2_GetComponentToWorld` (`self.DropLocation`)) "Undefined" "OverrideRootScale" null `DataTable To Drop` null))

(fn `DisableMouse`
  (bind _gamehud_reference (`self.GameHud Reference`))
  (set `/Game/Widget/GameHUD.InventoryVIsible` "Hidden" _gamehud_reference)
  (set `/Game/Widget/GameHUD.CrossHairVisible` "Visible" _gamehud_reference)
  (set `PlayerController.bShowMouseCursor` false (`GameplayStatics.GetPlayerController` 0))
  (`self.SetMovable` true))

(fn `DoRepair`
  (params (Part :type "EModular Enum" :default "EHead") (RepairValue :type "Float (double-precision)"))
  (`parent.DoRepair` Part RepairValue))

(fn `EnableMouse`
  (bind _gamehud_reference (`self.GameHud Reference`))
  (set `/Game/Widget/GameHUD.InventoryVIsible` "Visible" _gamehud_reference)
  (set `/Game/Widget/GameHUD.CrossHairVisible` "Hidden" _gamehud_reference)
  (set `PlayerController.bShowMouseCursor` true (`GameplayStatics.GetPlayerController` 0))
  (`self.SetMovable` false))

(fn `RefreshModularParts`
  (`parent.RefreshModularParts`)
  (`/Game/BluePrint/BP_UIPlayerPreView.SetSKM` (`self.PreviewActor`) (`self.ModularInventory`)))

(fn `UserConstructionScript`
  (`SkinnedMeshComponent.SetLeaderPoseComponent` (`self.SKM_BackAccessory`) (`self.SKM_UpperBody`) false)
  (`SkinnedMeshComponent.SetLeaderPoseComponent` (`self.SKM_LowerBody`) (`self.SKM_UpperBody`) false)
  (`SkinnedMeshComponent.SetLeaderPoseComponent` (`self.SKM_Head`) (`self.SKM_UpperBody`) false)
  (`SkinnedMeshComponent.SetLeaderPoseComponent` (`self.SKM_FaceAccessory`) (`self.SKM_UpperBody`) false)
  (`SkinnedMeshComponent.SetLeaderPoseComponent` (`self.SKM_LeftArm`) (`self.SKM_UpperBody`) false)
  (`SkinnedMeshComponent.SetLeaderPoseComponent` (`self.SKM_RightArm`) (`self.SKM_UpperBody`) false))