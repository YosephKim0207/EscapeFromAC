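; BP_Character is a modular character whose body-part and accessory meshes follow the upper-body mesh's pose, set via master pose in the construction script.
; BoostEffect attaches a flame emitter to the back accessory's rocketpack socket and sets its beam target to the fire-end socket's location at spawn.
; EnableInventory and DisableInventory swap the HUD's inventory and crosshair visibility, toggle the mouse cursor and call SetMovable to lock or restore movement.
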(event `self.BoostEffect`
  ;[1 1 1] Boost Effect
  (bind _returnvalue (`GameplayStatics.SpawnEmitterAttached` "/Game/ImportContents/M5VFXVOL2/Particles/Reference/Candlefire/0_CandleFire_pt2.0_CandleFire_pt2" (`self.SKM_BackAccessory`) "attach_rocketpack" (0.0 0.0 0.0) (struct) (6.0 4.0 1.0) "SnapToTargetIncludingScale"))
  (if (`KismetSystemLibrary.IsValid` _returnvalue)
    (`ParticleSystemComponent.SetBeamTargetPoint` _returnvalue 0 (`SceneComponent.GetSocketLocation` (`self.Mesh`) "attach_fireend") 0)))

(fn `DisableInventory`
  (bind _gamehud_reference (`self.GameHUD Reference`))
  (set `/Game/Widget/GameHUD.InventoryVIsible` "Hidden" _gamehud_reference)
  (set `/Game/Widget/GameHUD.CrossHairVisible` "Visible" _gamehud_reference)
  (set `PlayerController.bShowMouseCursor` false (`GameplayStatics.GetPlayerController` 0))
  (`self.SetMovable` true))

(fn `EnableInventory`
  (bind _gamehud_reference (`self.GameHUD Reference`))
  (set `/Game/Widget/GameHUD.InventoryVIsible` "Visible" _gamehud_reference)
  (set `/Game/Widget/GameHUD.CrossHairVisible` "Hidden" _gamehud_reference)
  (set `PlayerController.bShowMouseCursor` true (`GameplayStatics.GetPlayerController` 0))
  (`self.SetMovable` false))

(fn `UserConstructionScript`
  (`SkinnedMeshComponent.SetLeaderPoseComponent` (`self.SKM_LowerBody`) (`self.SKM_UpperBody`) false)
  (`SkinnedMeshComponent.SetLeaderPoseComponent` (`self.SKM_BackAccessory`) (`self.SKM_UpperBody`) false)
  (`SkinnedMeshComponent.SetLeaderPoseComponent` (`self.SKM_Head`) (`self.SKM_UpperBody`) false)
  (`SkinnedMeshComponent.SetLeaderPoseComponent` (`self.SKM_FaceAccessory`) (`self.SKM_UpperBody`) false)
  (`SkinnedMeshComponent.SetLeaderPoseComponent` (`self.SKM_LeftArm`) (`self.SKM_UpperBody`) false)
  (`SkinnedMeshComponent.SetLeaderPoseComponent` (`self.SKM_RightArm`) (`self.SKM_UpperBody`) false))