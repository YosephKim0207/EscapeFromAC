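; BP_PlayerController is a player controller that creates the game HUD and keeps a reference to the BP_Player character.
; On BeginPlay it caches the player character, then adds the GameHUD widget to the viewport, while a RefreshUIPlayerReference event re-caches the reference from the controlled pawn.
; InventoryCheck rebuilds the list of empty UserInventory slot indices, treating entries without a valid DataTable as empty, and returns whether any exist.
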(event `self.ReceiveBeginPlay`
  (bind _asbp_player (cast `/Game/BluePrint/BP_Player` (`GameplayStatics.GetPlayerCharacter` 0)))
  (set `self.PlayerReference` _asbp_player)
  (bind _returnvalue (`|CreateWidget` "/Game/Widget/GameHUD.GameHUD_C"))
  (bind _output_get (set `self.GameHUDReference` _returnvalue))
  (`UserWidget.AddToViewport` _output_get 0))

(event `Refresh UI Player Reference`
  (bind _asbp_player (cast `/Game/BluePrint/BP_Player` (`self.K2_GetPawn`)))
  (set `self.PlayerReference` _asbp_player))

(fn `Inventory Check`
  (returns (InventoryHasSpace :type Boolean))
  ;[1 1 1] Inventory Check
  (`KismetArrayLibrary.Array_Clear` (`self.EmptySlot`))
  (for (_array_element _array_index) (`self.UserInventory`)
    (if (not (`KismetSystemLibrary.IsValid` (`.DataTable` (break `DataTableRowHandle` _array_element))))
      (`KismetArrayLibrary.Array_Add` (`self.EmptySlot`) _array_index)))
  (return (> (`KismetArrayLibrary.Array_Length` (`self.EmptySlot`)) 0)))

(fn `UserConstructionScript`)