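; BP_UIPlayerPreView renders a modular-character preview of its owning BP_Player, apparently for UI display.
; On BeginPlay, its scene capture gets a new render target, fed into a dynamic material that is stored on the player.
; The construction script makes head, arm and lower-body meshes follow the upper body's pose.
; SetSKM resolves modular inventory items through two data-table lookups and swaps each body part's skeletal mesh.
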(event `self.ReceiveBeginPlay`
  ;[1 1 1] BeginPlay
  (bind _asbp_player (cast `/Game/BluePrint/BP_Player` (`self.GetOwner`))
    (:`then`
      (bind _returnvalue (`KismetRenderingLibrary.CreateRenderTarget2D` 256))
      (bind _output_get (set `SceneCaptureComponent2D.TextureTarget` _returnvalue (`self.SceneCaptureComponent2D`)))
      (bind _returnvalue_2 (`KismetMaterialLibrary.CreateDynamicMaterialInstance` "/Game/BluePrint/UI/RenderTarget_Mat.RenderTarget_Mat" (`KismetStringLibrary.Conv_StringToName` (`KismetStringLibrary.Concat_StrStr` (`KismetSystemLibrary.GetDisplayName` _asbp_player) (`KismetStringLibrary.Conv_IntToString` (`KismetMathLibrary.RandomInteger` 1000))))))
      (set `/Game/BluePrint/BP_Player.RenderTargetMat` _returnvalue_2 _asbp_player)
      (`MaterialInstanceDynamic.SetTextureParameterValue` _returnvalue_2 "RenderTexture" _output_get))
    (:`CastFailed`
      (`KismetSystemLibrary.PrintString` "UIPlayerPreview Cast Player Fail!"))))

(fn `SetSKM`
  (params (ModularInventory :type "Array of DataTableRowHandle Structure (by ref)"))
  (for _array_element ModularInventory
    (bind (_datatable _rowname) (break `DataTableRowHandle` _array_element))
    (if (`KismetSystemLibrary.IsValid` _datatable)
      (bind _returnvalue (`|GetDataTableRow` _datatable _rowname)
        (:`then`
          (bind (_itemimage _pickuptext _actiontext _itemtype _selectitemstatdatatable) (break `PickupItemData` _returnvalue))
          (if (`|EnumEquality` _itemtype "EModular")
            (bind (_datatable_2 _rowname_2) (break `DataTableRowHandle` _selectitemstatdatatable))
            (bind _returnvalue_2 (`|GetDataTableRow` _datatable_2 _rowname_2)
              (:`then`
                (bind (_skeletalmesh _parts) (break `ModularItemStatData` _returnvalue_2))
                (switch `EModular` _parts
                  (:`EHead`
                    (`SkinnedMeshComponent.SetSkinnedAssetAndUpdate` (`self.SKMHead`) _skeletalmesh true))
                  (:`ELeftArm`
                    (`SkinnedMeshComponent.SetSkinnedAssetAndUpdate` (`self.SKMLeftArm`) _skeletalmesh true))
                  (:`ERightArm`
                    (`SkinnedMeshComponent.SetSkinnedAssetAndUpdate` (`self.SKMRightArm`) _skeletalmesh true))
                  (:`EUpperBody`
                    (`SkinnedMeshComponent.SetSkinnedAssetAndUpdate` (`self.SKMUpperBody`) _skeletalmesh true))
                  (:`ELowerBody`
                    (`SkinnedMeshComponent.SetSkinnedAssetAndUpdate` (`self.SKMLowerBody`) _skeletalmesh true)))))))))))

(fn `UserConstructionScript`
  (`SkinnedMeshComponent.SetLeaderPoseComponent` (`self.SKMLowerBody`) (`self.SKMUpperBody`) false)
  (`SkinnedMeshComponent.SetLeaderPoseComponent` (`self.SKMLeftArm`) (`self.SKMUpperBody`) false)
  (`SkinnedMeshComponent.SetLeaderPoseComponent` (`self.SKMRightArm`) (`self.SKMUpperBody`) false)
  (`SkinnedMeshComponent.SetLeaderPoseComponent` (`self.SKMHead`) (`self.SKMUpperBody`) false))