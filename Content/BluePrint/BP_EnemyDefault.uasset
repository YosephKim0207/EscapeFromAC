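; BP_EnemyDefault is a default enemy Blueprint with a modular skeletal-mesh body and a drop inventory.
; The construction script makes the upper body mesh the master pose for the lower body, head, arms and accessory meshes, so all parts share its animation.
; On BeginPlay, it fills DropInventory with empty data table row handles based on DropInventoryVolume, then prints the resulting length.
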(event `self.ReceiveBeginPlay`
  (for _ (range (+ (`self.DropInventoryVolume`) 1))
    (`KismetArrayLibrary.Array_Add` (`self.DropInventory`) (make `DataTableRowHandle` null)))
  (`KismetSystemLibrary.PrintString` (`KismetStringLibrary.Conv_IntToString` (`KismetArrayLibrary.Array_Length` (`self.DropInventory`)))))

(fn `UserConstructionScript`
  (`SkinnedMeshComponent.SetLeaderPoseComponent` (`self.SKM_LowerBody`) (`self.SKM_UpperBody`) false)
  (`SkinnedMeshComponent.SetLeaderPoseComponent` (`self.SKM_BackAccessory`) (`self.SKM_UpperBody`) false)
  (`SkinnedMeshComponent.SetLeaderPoseComponent` (`self.SKM_Head`) (`self.SKM_UpperBody`) false)
  (`SkinnedMeshComponent.SetLeaderPoseComponent` (`self.SKM_FaceAccessory`) (`self.SKM_UpperBody`) false)
  (`SkinnedMeshComponent.SetLeaderPoseComponent` (`self.SKM_LeftArm`) (`self.SKM_UpperBody`) false)
  (`SkinnedMeshComponent.SetLeaderPoseComponent` (`self.SKM_RightArm`) (`self.SKM_UpperBody`) false))