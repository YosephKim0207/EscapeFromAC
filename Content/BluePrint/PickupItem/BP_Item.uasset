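; BP_Item is a pickup item Blueprint meant to take its mesh and material from a data table row chosen by SelectItemData.
; In SetItemOut, an IsBag branch looks up the row and applies StaticMesh and Material to the StaticMeshComponent, with matching steps on both sides.
; That logic is disconnected from the function entry, so it never executes, and the construction script is empty.
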(fn `Set Item Out `)

(fn `UserConstructionScript`)