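; BP_Bag is a bag pickup item that carries its own inventory.
; On BeginPlay it fills BagInventory with empty "None" data table row handles in a loop sized by BagVolume, then prints the resulting slot count.
; The item outline is set in both the Construction Script and BeginPlay through a SetItemOutline override that only calls the parent implementation.
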(event `self.ReceiveBeginPlay`
  (`self.SetItemOutline`)
  (for _ (range (+ (`self.BagVolume`) 1))
    (`KismetArrayLibrary.Array_Add` (`self.BagInventory`) (make `DataTableRowHandle` null)))
  (`KismetSystemLibrary.PrintString` (`KismetStringLibrary.Conv_IntToString` (`KismetArrayLibrary.Array_Length` (`self.BagInventory`)))))

(fn `SetItemOutline`
  (`parent.SetItemOutline`))

(fn `UserConstructionScript`
  (`self.SetItemOutline`))