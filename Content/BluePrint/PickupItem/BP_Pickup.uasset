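; Pickup item actor that, when picked up, places its data table row handle in the player's inventory and destroys itself.
; On BeginPlay it applies the parent's item outline, caches the player controller and loads its item data from the selected row.
; CallPickUp requires range and collision, writes to the first listed empty slot, then refreshes the HUD and garage inventory menus.
; DropAction is an empty stub.
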(event `self.ReceiveBeginPlay`
  (bind (_datatable _rowname) (break `DataTableRowHandle` (`self.SelectItemDataTable`)))
  ;[1 1 1] Begin Play
  (`self.SetItemOutline`)
  (bind _asbp_player_controller (cast `/Game/BluePrint/BP_PlayerController` (`GameplayStatics.GetPlayerController` 0)))
  (set `self.PlayerControllerReference` _asbp_player_controller)
  (bind _returnvalue (`|GetDataTableRow` _datatable _rowname)
    (:`then`
      (setmembers `PickupItemData` :`StructRef` _returnvalue))))

(event `CallPickUp`
  (bind _playercontrollerreference (`self.PlayerControllerReference`))
  (bind _gamehudreference (`/Game/BluePrint/BP_PlayerController.GameHUDReference` (`self.PlayerControllerReference`)))
  ;[1 1 1] Call PickUp
  (if (and (`self.bIsInRange`) (`self.GetActorEnableCollision`))
    (`KismetArrayLibrary.Array_Set` (`/Game/BluePrint/BP_PlayerController.UserInventory` _playercontrollerreference) (`|GetArrayItem` (`/Game/BluePrint/BP_PlayerController.EmptySlot` _playercontrollerreference)) (`self.SelectItemDataTable`))
    (`/Game/Widget/Inventory.RefreshInventory` (`/Game/Widget/GameHUD.InventoryMenu` _gamehudreference))
    (`/Game/Widget/GarageInventoryMenu.RefreshInventory` (`/Game/Widget/Garage.GarageInventoryMenu` (`/Game/Widget/GameHUD.Garage` _gamehudreference)))
    (`self.K2_DestroyActor`)))

(fn `Drop Action`
  (params (`DataTable To Drop` :type "DataTableRowHandle Structure"))
  (return))

(fn `SetItemOutline`
  (`parent.SetItemOutline`))

(fn `UserConstructionScript`
  (`self.SetItemOutline`))